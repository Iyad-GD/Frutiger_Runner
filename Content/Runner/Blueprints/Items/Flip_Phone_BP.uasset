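; Flip phone launch trap for the runner: overlapping its box plays a timeline that throws the character straight upward.
; The PhoneFlipping timeline's Launch Character event track launches the player character cached at BeginPlay, once per overlapping third-person character.
; The top half's rotation is lerped from the timeline track only on Finished, not per update, followed by a delayed reverse.
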(event OnComponentBeginOverlap(Box)
  (params (OverlappedComponent :type Primitive%20Component%20Object%20Reference) (OtherActor :type Actor%20Object%20Reference) (OtherComp :type Primitive%20Component%20Object%20Reference) (OtherBodyIndex :type Integer) (bFromSweep :type Boolean) (SweepResult :type Hit%20Result%20Structure%20%28by%20ref%29))
  (bind _main_track (Timeline|Phone%20Flipping Play)
    (:Finished
      (Transformation|SetRelativeRotation (Variables|Default|GetTop_Phone) (Math|Rotator|Lerp(Rotator) "0.000000,-90.000000,120.000000" "0.000000,-90.000000,-30.000000" _main_track) false false)
      (Utilities|FlowControl|Delay 5.0)
      (Timeline|Phone%20Flipping Reverse))
    (:Launch%20Character
      (for _array_element (Collision|GetOverlappingActors (Variables|Default|GetBox) "/Game/ThirdPerson/Blueprints/BP_ThirdPersonCharacter.BP_ThirdPersonCharacter_C" :!class /Script/Engine.PrimitiveComponent)
        (Character|LaunchCharacter (Variables|Default|GetAs%20BP%20Third%20Person%20Character) "0.000000,0.000000,1500.000000" true true)))))

(event EventBeginPlay
  (bind _asbp_third_person_character (Utilities|Casting|CastToBP_ThirdPersonCharacter (Game|GetPlayerCharacter 0)))
  (Variables|Default|SetAs%20BP%20Third%20Person%20Character _asbp_third_person_character))

(event Collision|EventActorBeginOverlap
  (params (OtherActor :type Actor%20Object%20Reference)))

(event EventTick
  (params (DeltaSeconds :type Float%20%28single-precision%29)))

(event EventTestCalling)

(fn ConstructionScript)