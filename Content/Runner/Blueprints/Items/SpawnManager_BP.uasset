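; Spawn manager for the runner that periodically spawns random obstacles or items from SpawnableObjects.
; A looping BeginPlay timer calls SpawnObjects, which places a random class at a random BP_SpawnPoint transform.
; Every Tick scans Objects_To_Spawn actors for any trailing the player beyond CleanupDistance on X.
; That cleanup check calls DestroyActor without a target, so it destroys the manager rather than the trailing actor.
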(event EventBeginPlay
  (Utilities|Time|SetTimerbyFunctionName 0 "SpawnObjects" (Variables|Default|GetSpawn%20Interval) true))

(event Collision|EventActorBeginOverlap
  (params (OtherActor :type Actor%20Object%20Reference)))

(event EventTick
  (params (DeltaSeconds :type Float%20%28single-precision%29))
  ;[0.15 0.15 0.15 0.5] Cleanup
  (Variables|Default|SetPlayerLocVar (Transformation|GetActorLocation (Game|GetPlayerCharacter 0)))
  (bind _outactors (Actor|GetAllActorsOfClass "/Game/Runner/Blueprints/Items/Objects_To_Spawn.Objects_To_Spawn_C"))
  (for _array_element _outactors
    (if (> (- (.x (Variables|Default|GetPlayerLocVar)) (.x (Transformation|GetActorLocation _array_element))) (Variables|Default|GetCleanupDistance))
      (Actor|DestroyActor))))

(fn ConstructionScript)

(fn SpawnObjects
  (bind _spawnable_objects (Variables|Default|GetSpawnable%20Objects))
  (bind _outactors (Actor|GetAllActorsOfClass "/Game/Runner/Blueprints/Items/BP_SpawnPoint.BP_SpawnPoint_C"))
  (bind _output_get (Variables|Default|SetSpawn%20Points _outactors))
  (Game|SpawnActorfromClass (Utilities|Array|Get(acopy) _spawnable_objects (Math|Random|RandomIntegerinRange 0 (- (Utilities|Array|Length _spawnable_objects) 1))) (Transformation|GetActorTransform (Utilities|Array|Get(acopy) _output_get (Math|Random|RandomIntegerinRange 0 (- (Utilities|Array|Length _output_get) 1)))) "AdjustIfPossibleButAlwaysSpawn" "MultiplyWithRoot" 0 0))