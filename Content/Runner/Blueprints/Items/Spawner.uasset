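; Runner item spawner that builds a spiral of randomly chosen platform Blueprints when play begins.
; A single loop spawns Count actors, stepping forward along Y while cosine and sine of a stepped angle place each in the XZ plane.
; The radius interpolates from start toward end across the loop, and positions are absolute rather than offset from the spawner.
; Spawns adjust for collisions but always succeed.
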(event EventBeginPlay
  (for _index (range 0 (- (Variables|Default|GetCount) 1))
    (Game|SpawnActorfromClass (.OutItem (Utilities|Array|Random (Variables|Default|GetBPs%20To%20Spawn))) (Math|Transform|MakeTransform (Math|Vector|MakeVector (* (Math|Trig|Cos(Degrees) (* (Math|Conversions|ToFloat(Integer) _index) (Variables|Default|GetAngle%20Step))) (Math|Float|Lerp (Variables|Default|GetRadius%20Start) (Variables|Default|GetRadius%20End) (/ (Math|Conversions|ToFloat(Integer) _index) (Variables|Default|GetCount)))) (* (Math|Conversions|ToFloat(Integer) _index) (Variables|Default|GetForward%20Step)) (* (Math|Float|Lerp (Variables|Default|GetRadius%20Start) (Variables|Default|GetRadius%20End) (/ (Math|Conversions|ToFloat(Integer) _index) (Variables|Default|GetCount))) (Math|Trig|Sin(Degrees) (* (Math|Conversions|ToFloat(Integer) _index) (Variables|Default|GetAngle%20Step))))) "0, 0, 0" "1.000000,1.000000,1.000000") "AdjustIfPossibleButAlwaysSpawn" "MultiplyWithRoot" 0 0)))

(fn ConstructionScript)