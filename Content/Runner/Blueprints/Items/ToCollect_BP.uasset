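; Collectible pickup for the runner that reacts when the third-person player character touches it.
; Box overlap by that character calls CollectionInteraction, whose logic is not in this graph, then destroys the actor.
; BeginPlay caches the player; Tick offsets the RotatingMovement pivot when the player's world X and Y are near the pivot translation value.
; That proximity test compares against the pivot offset rather than the pickup's location, and the offset is never reset.
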(event OnComponentBeginOverlap(Box)
  (params (OverlappedComponent :type Primitive%20Component%20Object%20Reference) (OtherActor :type Actor%20Object%20Reference) (OtherComp :type Primitive%20Component%20Object%20Reference) (OtherBodyIndex :type Integer) (bFromSweep :type Boolean) (SweepResult :type Hit%20Result%20Structure%20%28by%20ref%29))
  (Utilities|Casting|CastToBP_ThirdPersonCharacter OtherActor)
  (CallFunction|CollectionInteraction)
  (Actor|DestroyActor))

(event EventBeginPlay
  (bind _asbp_third_person_character (Utilities|Casting|CastToBP_ThirdPersonCharacter (Game|GetPlayerCharacter 0)))
  (Variables|Default|SetPlayerRef _asbp_third_person_character))

(event Collision|EventActorBeginOverlap
  (params (OtherActor :type Actor%20Object%20Reference)))

(event EventTick
  (params (DeltaSeconds :type Float%20%28single-precision%29))
  (bind _rotatingmovement (Variables|Default|GetRotatingMovement))
  (bind _playerref (Variables|Default|GetPlayerRef))
  (bind _returnvalue (Transformation|GetActorTransform _playerref))
  (if (and (< (Math|Float|Absolute(Float) (- (.x (.location _returnvalue)) (.x (Variables|/Script/Engine.RotatingMovementComponent|GetPivotTranslation _rotatingmovement)))) 5e+02) (< (Math|Float|Absolute(Float) (- (.y (.location _returnvalue)) (.y (Variables|/Script/Engine.RotatingMovementComponent|GetPivotTranslation _rotatingmovement)))) 5e+02))
    (Variables|/Script/Engine.RotatingMovementComponent|SetPivotTranslation _rotatingmovement (Math|Vector|MakeVector 0.0 1e+02 1e+02))))

(fn ConstructionScript)