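; BP_SpawnPoint is a spawn point actor that circles a platform in the runner game.
; On BeginPlay it finds the Platform_BP actor and keeps it as the center.
; Each Tick it sets its location from the sine and cosine of game time scaled by RotationSpeed, tracing a horizontal orbit of the given Radius at the platform's height, without sweeping.
; The file itself contains no spawning logic.
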(event EventBeginPlay
  (bind _returnvalue (Actor|GetActorOfClass "/Game/Runner/Blueprints/Items/Platform_BP.Platform_BP_C"))
  (Variables|Default|SetCenter%20Actor _returnvalue))

(event Collision|EventActorBeginOverlap
  (params (OtherActor :type Actor%20Object%20Reference)))

(event EventTick
  (params (DeltaSeconds :type Float%20%28single-precision%29))
  (bind _returnvalue (Utilities|Time|GetGameTimeinSeconds))
  (bind _rotation_speed (Variables|Default|GetRotation%20Speed))
  (bind _radius (Variables|Default|GetRadius))
  (bind _center_actor (Variables|Default|GetCenter%20Actor))
  (bind _returnvalue_2 (Transformation|GetActorLocation _center_actor))
  (bind _returnvalue_3 (* _returnvalue _rotation_speed))
  (Transformation|SetActorLocation (Math|Vector|MakeVector (+ (.x _returnvalue_2) (* (Math|Trig|Cos(Radians) _returnvalue_3) _radius)) (+ (.y _returnvalue_2) (* _radius (Math|Trig|Sin(Radians) _returnvalue_3))) (.z _returnvalue_2)) false false))

(fn ConstructionScript)