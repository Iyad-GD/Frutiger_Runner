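; ObjectsTrigger is a runner-game trigger actor that starts and stops the player character's object pivot rotation.
; When the player character overlaps its Box, it sends ObjectsPivotRotationMessage to that character.
; Each Tick it compares the Box's world Y with the cached player's Y, sending ObjectPivotStopMessage whenever the player's Y is greater.
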(event OnComponentBeginOverlap(Box)
  (params (OverlappedComponent :type Primitive%20Component%20Object%20Reference) (OtherActor :type Actor%20Object%20Reference) (OtherComp :type Primitive%20Component%20Object%20Reference) (OtherBodyIndex :type Integer) (bFromSweep :type Boolean) (SweepResult :type Hit%20Result%20Structure%20%28by%20ref%29))
  (bind _asbp_third_person_character (Utilities|Casting|CastToBP_ThirdPersonCharacter OtherActor))
  (Class|Interactions|ObjectsPivotRotation(Message) _asbp_third_person_character))

(event EventBeginPlay
  (bind _asbp_third_person_character (Utilities|Casting|CastToBP_ThirdPersonCharacter (Game|GetPlayerCharacter 0)))
  (Variables|Default|SetChar%20Ref _asbp_third_person_character))

(event EventTick
  (params (DeltaSeconds :type Float%20%28single-precision%29))
  (bind _char_ref (Variables|Default|GetChar%20Ref))
  (if (< (- (.y (Transformation|GetWorldLocation (Variables|Default|GetBox))) (.y (Transformation|GetActorLocation _char_ref))) 0.0)
    (Class|Interactions|ObjectPivotStop(Message) _char_ref)))

(fn ConstructionScript)